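; Decorative traffic light actor that randomly switches its red, amber and green lamps.
; The construction script creates three dynamic material instances, caches their default brightness and emissive color, and starts on red.
; Tick feeds a random-length Delay, then rolls each lamp separately, so several or none can be lit.
; ChangeLights restores cached values for lit lamps and dims unlit ones through material parameters.
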(event EventBeginPlay)

(event Collision|EventActorBeginOverlap
  (params (OtherActor :type Actor%20Object%20Reference)))

(event EventTick
  (params (DeltaSeconds :type Float%20%28single-precision%29))
  (bind _returnvalue (Math|Random|RandomIntegerinRange 0 2))
  (Utilities|FlowControl|Delay (Math|Random|RandomFloatinRange (Variables|Default|GetMin_Interval) (Variables|Default|GetMax_Interval)))
  (CallFunction|ChangeLights (Utilities|Select :Index _returnvalue :Option%200 true :Option%201 false :Option%202 false) (Utilities|Select :Index _returnvalue :Option%200 false :Option%201 true :Option%202 false) (Utilities|Select :Index _returnvalue :Option%200 false :Option%201 false :Option%202 true)))

(fn ConstructionScript
  (bind _staticmeshcomponent (Variables|Debug|GetStaticMeshComponent))
  (Utilities|FlowControl|Sequence
    (:then_0
      (bind _returnvalue (Rendering|Material|CreateDynamicMaterialInstance _staticmeshcomponent 2 "/Game/Materials/Obstacles/MI_Semaforo_Luz_Rojo.MI_Semaforo_Luz_Rojo" "Rojo" :!class /Script/Engine.PrimitiveComponent))
      (bind _output_get (Variables|Default|SetRojo _returnvalue))
      (Utilities|FlowControl|Sequence
        (:then_0
          (bind _returnvalue_2 (Rendering|Material|GetScalarParameterValue _output_get "Brightness" :!class /Script/Engine.MaterialInstanceDynamic))
          (Variables|Default|SetDefault_red _returnvalue_2))
        (:then_1
          (bind _returnvalue_3 (Rendering|Material|GetVectorParameterValue _output_get "Color/Emissive" :!class /Script/Engine.MaterialInstanceDynamic))
          (Variables|Default|SetColor_Red _returnvalue_3))))
    (:then_1
      (bind _returnvalue_4 (Rendering|Material|CreateDynamicMaterialInstance _staticmeshcomponent 3 "/Game/Materials/Obstacles/MI_Semaforo_Luz_Ambar.MI_Semaforo_Luz_Ambar" "Ambar" :!class /Script/Engine.PrimitiveComponent))
      (bind _output_get_2 (Variables|Default|SetAmbar _returnvalue_4))
      (Utilities|FlowControl|Sequence
        (:then_0
          (bind _returnvalue_5 (Rendering|Material|GetScalarParameterValue _output_get_2 "Brightness" :!class /Script/Engine.MaterialInstanceDynamic))
          (Variables|Default|SetDefault_yellow _returnvalue_5))
        (:then_1
          (bind _returnvalue_6 (Rendering|Material|GetVectorParameterValue _output_get_2 "Color/Emissive" :!class /Script/Engine.MaterialInstanceDynamic))
          (Variables|Default|SetColor_Yellow _returnvalue_6))))
    (:then_2
      (bind _returnvalue_7 (Rendering|Material|CreateDynamicMaterialInstance _staticmeshcomponent 4 "/Game/Materials/Obstacles/MI_Semaforo_Luz_Verde.MI_Semaforo_Luz_Verde" "Verde" :!class /Script/Engine.PrimitiveComponent))
      (bind _output_get_3 (Variables|Default|Setverde _returnvalue_7))
      (Utilities|FlowControl|Sequence
        (:then_0
          (bind _returnvalue_8 (Rendering|Material|GetScalarParameterValue _output_get_3 "Brightness" :!class /Script/Engine.MaterialInstanceDynamic))
          (Variables|Default|SetDefault_green _returnvalue_8))
        (:then_1
          (bind _returnvalue_9 (Rendering|Material|GetVectorParameterValue _output_get_3 "Color/Emissive" :!class /Script/Engine.MaterialInstanceDynamic))
          (Variables|Default|SetColor_Green _returnvalue_9))))
    (:then_3
      (CallFunction|ChangeLights true false false))))

(fn ChangeLights
  (params (Red :type Boolean) (Yellow :type Boolean) (Green :type Boolean))
  (bind _color_green (Variables|Default|GetColor_Green))
  (bind _rojo (Variables|Default|GetRojo))
  (bind _ambar (Variables|Default|GetAmbar))
  (bind _verde (Variables|Default|Getverde))
  (bind _color_red (Variables|Default|GetColor_Red))
  (bind _color_yellow (Variables|Default|GetColor_Yellow))
  (Utilities|FlowControl|Sequence
    (:then_0
      (Rendering|Material|SetScalarParameterValue _rojo "Brightness" (Math|Float|SelectFloat (Variables|Default|GetDefault_red) -1.0 Red) :!class /Script/Engine.MaterialInstanceDynamic)
      (Rendering|Material|SetVectorParameterValue _rojo "Color/Emissive" (Math|Color|SelectColor _color_red (* _color_red 0.1) Red) :!class /Script/Engine.MaterialInstanceDynamic))
    (:then_1
      (Rendering|Material|SetScalarParameterValue _ambar "Brightness" (Math|Float|SelectFloat (Variables|Default|GetDefault_yellow) -1.0 Yellow) :!class /Script/Engine.MaterialInstanceDynamic)
      (Rendering|Material|SetVectorParameterValue _ambar "Color/Emissive" (Math|Color|SelectColor _color_yellow (* _color_yellow 0.3) Yellow) :!class /Script/Engine.MaterialInstanceDynamic))
    (:then_2
      (Rendering|Material|SetScalarParameterValue _verde "Brightness" (Math|Float|SelectFloat (Variables|Default|GetDefault_green) -1.0 Green) :!class /Script/Engine.MaterialInstanceDynamic)
      (Rendering|Material|SetVectorParameterValue _verde "Color/Emissive" (Math|Color|SelectColor _color_green (* _color_green 0.1) Green) :!class /Script/Engine.MaterialInstanceDynamic))))