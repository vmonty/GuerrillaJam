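; BP_sewer is a sewer actor with a crocodile that bites while the player is near.
; Box1 begin overlap with BP_Player sets DoBite on the crocodile's Cocotrilo_AnimBP and plays a timeline that moves Cylinder1's relative location.
; Leaving Box2 clears DoBite after a short delay and reverses the timeline from its end.
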(event OnComponentBeginOverlap(Box1)
  (params (OverlappedComponent :type Primitive%20Component%20Object%20Reference) (OtherActor :type Actor%20Object%20Reference) (OtherComp :type Primitive%20Component%20Object%20Reference) (OtherBodyIndex :type Integer) (bFromSweep :type Boolean) (SweepResult :type Hit%20Result%20Structure%20%28by%20ref%29))
  (Utilities|Casting|CastToBP_Player OtherActor)
  (bind _ascocotrilo_anim_bp (Utilities|Casting|CastToCocotrilo_AnimBP (Components|SkeletalMesh|GetAnimInstance (Variables|Default|GetCocodrilo))))
  (Variables|/Game/Animation/Cocotrilo_AnimBP.Cocotrilo_AnimBP_C|SetDoBite _ascocotrilo_anim_bp true)
  (bind _alpha (Timeline|Timeline_0 PlayFromStart)
    (:Update
      (Transformation|SetRelativeLocation (Variables|Default|GetCylinder1) _alpha false false))))

(event OnComponentEndOverlap(Box2)
  (params (OverlappedComponent :type Primitive%20Component%20Object%20Reference) (OtherActor :type Actor%20Object%20Reference) (OtherComp :type Primitive%20Component%20Object%20Reference) (OtherBodyIndex :type Integer))
  (Utilities|Casting|CastToBP_Player OtherActor)
  (Utilities|FlowControl|Delay 3.0)
  (bind _ascocotrilo_anim_bp (Utilities|Casting|CastToCocotrilo_AnimBP (Components|SkeletalMesh|GetAnimInstance (Variables|Default|GetCocodrilo))))
  (Variables|/Game/Animation/Cocotrilo_AnimBP.Cocotrilo_AnimBP_C|SetDoBite _ascocotrilo_anim_bp false)
  (bind _alpha (Timeline|Timeline_0 ReverseFromEnd)
    (:Update
      (Transformation|SetRelativeLocation (Variables|Default|GetCylinder1) _alpha false false))))

(event EventBeginPlay)

(event Collision|EventActorBeginOverlap
  (params (OtherActor :type Actor%20Object%20Reference)))

(event EventTick
  (params (DeltaSeconds :type Float%20%28single-precision%29)))

(fn ConstructionScript)