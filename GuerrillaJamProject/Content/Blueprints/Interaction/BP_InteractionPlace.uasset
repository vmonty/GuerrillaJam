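; BP_InteractionPlace is a mission trigger that completes when the player stands still inside it for a set time.
; Once enabled, Tick accumulates time while the overlapping BP_Player is nearly motionless, resetting it on movement or exit.
; The timer drives a WB_MissionRadialProgress widget.
; On completion it calls InteractionComplete once with itself and its MissionID, then destroys itself after a short delay.
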(event Custom|InteractionComplete_Event
  (params (InteractionPlace :type BP%20Interaction%20Place%20Object%20Reference) (MissionID :type Integer)))

(event EventBeginPlay
  (Variables|Default|SetIsInteractionComplete false)
  (CallFunction|ResetTimer))

(event Collision|EventActorBeginOverlap
  (params (OtherActor :type Actor%20Object%20Reference))
  (if (Variables|Default|GetActive)
    (bind _asbp_player (Utilities|Casting|CastToBP_Player OtherActor))
    (Variables|Default|SetPlayerInside true)
    (Development|PrintString "Player Inside")
    (Variables|Default|SetActorInside _asbp_player)))

(event EventTick
  (params (DeltaSeconds :type Float%20%28single-precision%29))
  (if (and (Variables|Default|GetPlayerInside) (Variables|Default|GetActive))
    (bind _actorinside (Variables|Default|GetActorInside)
      (:then
        (if (Math|Vector|Equal(Vector) (Transformation|GetVelocity _actorinside) "0, 0, 0" 0.1)
          (CallFunction|UpdateTimer DeltaSeconds)
          (Math|Float|CompareFloat (Variables|Default|GetTimePassed) (Variables|Default|GetTimeToComplete)
            (:>
              _)
            (:==
              _))
          (if (not (Variables|Default|GetIsInteractionComplete))
            (Variables|Default|SetIsInteractionComplete true)
            (Development|PrintString "Done")
            (Default|CallInteractionComplete self (Variables|Default|GetMissionID))
            (Utilities|FlowControl|Delay 0.2)
            (Actor|DestroyActor))
          (elif (!= 0.0 (Variables|Default|GetTimePassed))
            (CallFunction|ResetTimer))))
      (:else))))

(event Collision|EventActorEndOverlap
  (params (OtherActor :type Actor%20Object%20Reference))
  (if (Variables|Default|GetActive)
    (Utilities|Casting|CastToBP_Player OtherActor)
    (Variables|Default|SetPlayerInside false)
    (Development|PrintString "Player Outside")
    (Development|PrintString "ResetTimer")
    (Variables|Default|SetActorInside 0)
    (CallFunction|ResetTimer)))

(fn ConstructionScript)

(fn ResetTimer
  (Variables|Default|SetTimePassed 0.0)
  (CallFunction|UpdateSlider))

(fn UpdateTimer
  (params (DeltaTime :type Float%20%28single-precision%29))
  (Variables|Default|SetTimePassed (+ DeltaTime (Variables|Default|GetTimePassed)))
  (CallFunction|UpdateSlider)
  (return))

(fn UpdateSlider
  (bind _aswb_mission_radial_progress (Utilities|Casting|CastToWB_MissionRadialProgress (UserInterface|GetUserWidgetObject (Variables|Default|GetRadialProgressWidget))))
  (Default|UpdateProgress _aswb_mission_radial_progress (/ (Math|Float|Clamp(Float) (Variables|Default|GetTimePassed) 0.0 (Variables|Default|GetTimeToComplete)) (Variables|Default|GetTimeToComplete))))

(fn EnableTrigger
  (Variables|Default|SetActive true)
  (Rendering|SetActorHiddenInGame false))

(fn SetMissionID
  (params (NewParam :type Integer))
  (Variables|Default|SetMissionID NewParam))