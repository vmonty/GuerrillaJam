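; Traffic manager that moves a row of skeletal mesh vehicles along a spline, forward or backward.
; The construction script spawns a mesh component per VehicleArray entry, spacing them by cumulative PathOffset.X, with Y and Z as lateral and height offsets.
; Tick steps each stored world location (DistanceArray, despite its name) along the spline tangent and snaps it back to the spline.
; Speed applies per frame, ignoring delta time.
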(event EventBeginPlay)

(event Collision|EventActorBeginOverlap
  (params (OtherActor :type Actor%20Object%20Reference)))

(event EventTick
  (params (DeltaSeconds :type Float%20%28single-precision%29))
  (for (_array_element _array_index) (Variables|Default|GetVehicleArray)
    (CallFunction|UpdateVehiclePath _array_element _array_index DeltaSeconds)))

(fn ConstructionScript
  (CallFunction|InitializeTraffic))

(fn InitializeTraffic
  (bind _spline (Variables|Default|GetSpline))
  (for (_array_element _array_index) (Variables|Default|GetVehicleArray)
    (LocalVariables|SetVehicleLocal _array_element)
    (LocalVariables|SetIndexLocal _array_index)
    (Utilities|FlowControl|Sequence
      (:then_0
        (bind _returnvalue (AddComponent|AddSkeletalMeshComponent false))
        (bind _output_get (LocalVariables|SetComp _returnvalue))
        (Utilities|Array|SetArrayElem (LocalVariables|GetCompLocal) (LocalVariables|GetIndexLocal) _output_get true)
        (Class|SkinnedMeshComponent|SetSkeletalMesh _output_get (Utilities|Struct|BreakSTRUCT_TrafficElement (LocalVariables|GetVehicleLocal)) true))
      (:then_1
        (bind _output_get_2 (LocalVariables|SetDistanceTotal (+ (LocalVariables|GetDistanceTotal) (.x (Utilities|Struct|BreakSTRUCT_TrafficElement (LocalVariables|GetVehicleLocal))))))
        (Utilities|Array|SetArrayElem (LocalVariables|GetDistanceLocal) (LocalVariables|GetIndexLocal) (Spline|GetLocationatDistanceAlongSpline _spline _output_get_2 "World") true)
        (Transformation|SetWorldLocationAndRotation (LocalVariables|GetComp) (+ (Spline|GetLocationatDistanceAlongSpline _spline _output_get_2 "World") (* (Class|SplineComponent|GetRightVectoratDistanceAlongSpline _spline _output_get_2 "Local") (.y (Utilities|Struct|BreakSTRUCT_TrafficElement (LocalVariables|GetVehicleLocal)))) (Math|Vector|MakeVector 0.0 0.0 (.z (Utilities|Struct|BreakSTRUCT_TrafficElement (LocalVariables|GetVehicleLocal))))) (Math|Rotator|CombineRotators (Utilities|Select :Index (Variables|Default|GetDirection) :Forward "0, 0, 0" :Backward "0,-180.000000, 0") (Spline|GetRotationatDistanceAlongSpline _spline _output_get_2 "World")) false true))))
  (Variables|Default|SetCompArray (LocalVariables|GetCompLocal))
  (Variables|Default|SetDistanceArray (LocalVariables|GetDistanceLocal)))

(fn UpdateVehiclePath
  (params (Vehicle :type STRUCT%20Traffic%20Element%20Structure) (Index :type Integer) (Delta :type Float%20%28single-precision%29))
  (bind _spline (Variables|Default|GetSpline))
  (bind _direction (Variables|Default|GetDirection))
  (bind _spline_2 (Variables|Default|GetSpline))
  (bind _speed (Variables|Default|GetSpeed))
  (bind _distancearray (Variables|Default|GetDistanceArray))
  (bind _pathoffset (Utilities|Struct|BreakSTRUCT_TrafficElement Vehicle))
  (bind _output (Utilities|Array|Get(acopy) _distancearray Index))
  (bind _returnvalue (Utilities|Select :Index _direction :Forward 1.0 :Backward -1.0))
  (bind _returnvalue_2 (Spline|FindDirectionClosesttoWorldLocation _spline _output "World"))
  (bind _returnvalue_3 (Spline|FindLocationClosesttoWorldLocation _spline _output "World"))
  (bind _returnvalue_4 (* _speed _returnvalue))
  (bind _returnvalue_5 (* _returnvalue_2 _returnvalue_4))
  (bind _returnvalue_6 (+ _returnvalue_3 _returnvalue_5))
  (bind _returnvalue_7 (Spline|FindLocationClosesttoWorldLocation _spline_2 _returnvalue_6 "World"))
  (Utilities|Array|SetArrayElem (Variables|Default|GetDistanceArray) Index _returnvalue_7)
  (Transformation|SetWorldLocationAndRotation (Utilities|Array|Get(acopy) (Variables|Default|GetCompArray) Index) (+ _returnvalue_7 (* (Class|SplineComponent|FindRightVectorClosesttoWorldLocation _spline_2 _returnvalue_6 "World") (.y _pathoffset)) (Math|Vector|MakeVector 0.0 0.0 (.z _pathoffset))) (Math|Rotator|CombineRotators (Utilities|Select :Index _direction :Forward "0, 0, 0" :Backward "0,180.000000, 0") (Class|SplineComponent|FindRotationClosesttoWorldLocation _spline_2 _returnvalue_6 "World")) false true))