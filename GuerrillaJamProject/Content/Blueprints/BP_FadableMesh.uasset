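; BP_FadableMesh is an actor whose mesh can fade in and out through FadeIn_Mesh and FadeOut_Mesh events.
; The construction script creates a dynamic material instance from FadeableMaterial on slot 0.
; Separate timelines drive its Alpha scalar, played forward for fade-in and reversed for fade-out.
; IsFading blocks fade-in while set, but fade-out only toggles it without checking, and both timelines clear it on finish.
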(event Custom|FadeIn_Mesh
  (if (not (Variables|Default|GetisFading))
    (Variables|Default|SetisFading true)
    (bind _fade (Timeline|Timeline_0 PlayFromStart)
      (:Update
        (Rendering|Material|SetScalarParameterValue (Variables|Default|GetFadeableMat) "Alpha" _fade :!class /Script/Engine.MaterialInstanceDynamic))
      (:Finished
        (Variables|Default|SetisFading false)))))

(event Custom|FadeOut_Mesh
  (Variables|Default|SetisFading (not (Variables|Default|GetisFading)))
  (bind _fade (Timeline|Timeline_1 ReverseFromEnd)
    (:Update
      (Rendering|Material|SetScalarParameterValue (Variables|Default|GetFadeableMat) "Alpha" _fade :!class /Script/Engine.MaterialInstanceDynamic))
    (:Finished
      (Variables|Default|SetisFading false))))

(event EventBeginPlay)

(event Collision|EventActorBeginOverlap
  (params (OtherActor :type Actor%20Object%20Reference)))

(event EventTick
  (params (DeltaSeconds :type Float%20%28single-precision%29)))

(fn ConstructionScript
  (bind _returnvalue (Rendering|Material|CreateDynamicMaterialInstance (Variables|Default|GetMesh) 0 (Variables|Default|GetFadeableMaterial) "Alpha" :!class /Script/Engine.PrimitiveComponent))
  (Variables|Default|SetFadeableMat _returnvalue))