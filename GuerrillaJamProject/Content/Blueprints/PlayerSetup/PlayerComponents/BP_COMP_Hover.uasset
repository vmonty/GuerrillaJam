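; Hover component in the player setup that pushes a physics-simulated parent mesh upward when a trace detects a surface.
; InitComponent stores the mesh and enables physics; each tick runs a Visibility line trace from the component, its end computed by multiplying location by the scaled negative up vector rather than adding.
; On a hit, a local Z force fades from HoverForce toward zero with hit distance, and linear and angular damping are set.
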(event Custom|InitComponent
  (params (MeshComponent :type Mesh%20Component%20Object%20Reference))
  ;[1 1 1] Initialize
  (bind _output_get (Variables|Default|SetParentComp MeshComponent))
  (Physics|SetSimulatePhysics _output_get true))

(event EventBeginPlay)

(event EventTick
  (params (DeltaSeconds :type Float%20%28single-precision%29))
  (bind _returnvalue (Transformation|GetWorldLocation))
  (bind _parentcomp (Variables|Default|GetParentComp))
  (bind (_outhit _returnvalue_2) (Collision|LineTraceByChannel _returnvalue (* _returnvalue (* (Math|Vector|GetUpVector) (* (Variables|Default|GetTraceLength) -1.0))) "TraceTypeQuery1" false 0 "None"))
  (if _returnvalue_2
    (Class|PrimitiveComponent|AddForceatLocationLocal _parentcomp (Math|Vector|MakeVector 0.0 0.0 (Math|Float|Lerp (Variables|Default|GetHoverForce) 0.0 (/ (Math|Vector|VectorLength (- (.Location (Collision|BreakHitResult _outhit)) _returnvalue)) (Variables|Default|GetTraceLength)))) "0, 0, 0" "None")
    (Class|PrimitiveComponent|SetLinearDamping _parentcomp 3.0)
    (Class|PrimitiveComponent|SetAngularDamping _parentcomp 5.0)))