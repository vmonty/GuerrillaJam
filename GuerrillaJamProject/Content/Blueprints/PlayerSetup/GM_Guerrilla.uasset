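; Guerrilla game mode that owns the player's money and the countdown timers for missions, both shown in a mission time HUD widget.
; BeginPlay creates the widget and finds the mission manager; InitializeTimerWidget adds each mission's timer box and array entries.
; PlayTimer activates a timer by MissionID in parallel arrays.
; Tick decrements active timers, updates the widget and reports expired missions to the manager as failed.
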(event EventBeginPlay
  (Variables|Default|SetCurrentMoney (Variables|Default|GetBaseMoney))
  (bind _returnvalue (UserInterface|CreateWidget "/Game/UI/Widget_MissionTimeDisplay.Widget_MissionTimeDisplay_C" (Game|GetPlayerController 0) 9e+01 3 1 (Variables|Default|GetBaseMoney) (Variables|Default|GetMoneyIntegrals) (Variables|Default|GetMoneyDecimals)))
  (bind _output_get (Variables|Default|SetWidget_Timer _returnvalue))
  (UserInterface|Viewport|AddtoViewport _output_get 0)
  (CallFunction|UpdateMoney 0.0)
  (bind _outactors (Actor|GetAllActorsOfClass "/Game/Blueprints/Missions/BP_MissionManager.BP_MissionManager_C"))
  (bind _output_get_2 (Variables|Default|SetMissionManager (Utilities|Array|Get(acopy) _outactors)))
  (for _array_element (Variables|/Game/Blueprints/Missions/BP_MissionManager.BP_MissionManager_C|GetMissionList _output_get_2)
    _))

(event EventTick
  (params (DeltaSeconds :type Float%20%28single-precision%29))
  (bind _currenttime (Variables|Default|GetCurrentTime))
  (if (> (Variables|Default|GetTimersActiveAmmount) 0)
    (for (_array_element _array_index) (Variables|Default|GetTimerActive)
      (if _array_element
        (Utilities|Array|SetArrayElem _currenttime _array_index (- (Utilities|Array|Get(acopy) _currenttime _array_index) DeltaSeconds))
        (Math|Float|CompareFloat (Utilities|Array|Get(acopy) _currenttime _array_index) 0.0
          (:>
            (CallFunction|SetTimer (Utilities|Array|Get(acopy) (Variables|/Game/Blueprints/Missions/BP_MissionManager.BP_MissionManager_C|GetMissionList (Variables|Default|GetMissionManager)) _array_index) (Utilities|Array|Get(acopy) _currenttime _array_index)))
          (:==
            (Utilities|Array|SetArrayElem (Variables|Default|GetTimerActive) _array_index false :!label _label)
            (Default|MissionFailed (Variables|Default|GetMissionManager) (Utilities|Array|Get(acopy) (Variables|/Game/Blueprints/Missions/BP_MissionManager.BP_MissionManager_C|GetMissionList (Variables|Default|GetMissionManager)) _array_index)))
          (:<
            (goto _label)))))))

(fn ConstructionScript)

(fn UpdateMoney
  (params (DeltaFunds :type Float%20%28single-precision%29))
  (bind _output_get (Variables|Default|SetCurrentMoney (+ DeltaFunds (Variables|Default|GetCurrentMoney))))
  (Default|SetMoney (Variables|Default|GetWidget_Timer) _output_get))

(fn UpdateTimer)

(fn InitializeTimerWidget
  (params (Mission :type STRUCT%20Mission%20Settings%20Structure))
  (bind (_missionid _targetfood _targetclient _ordertime _ordercost _oderbenefit _odertype _orderstate _timerboxwidget) (Utilities|Struct|BreakSTRUCT_MissionSettings Mission))
  (bind _widget_timer (Variables|Default|GetWidget_Timer))
  (Widget|Panel|AddChild (Variables|/Game/UI/Widget_MissionTimeDisplay.Widget_MissionTimeDisplay_C|GetTimerBoxContainer _widget_timer) _timerboxwidget)
  (Default|SetMissionType _timerboxwidget _odertype)
  (Utilities|Array|Add (Variables|/Game/UI/Widget_MissionTimeDisplay.Widget_MissionTimeDisplay_C|GetTimerBoxList _widget_timer) _timerboxwidget)
  (Utilities|Array|Add (Variables|Default|GetTimerActive) false)
  (Utilities|Array|Add (Variables|Default|GetCurrentTime) _ordertime))

(fn PlayTimer
  (params (Mission :type STRUCT%20Mission%20Settings%20Structure))
  (bind _missionid (Utilities|Struct|BreakSTRUCT_MissionSettings Mission))
  (if (not (Utilities|Array|Get(acopy) (Variables|Default|GetTimerActive) _missionid))
    (Utilities|Array|SetArrayElem (Variables|Default|GetTimerActive) _missionid true)
    (Development|PrintString (Utilities|String|Append "Index: " (Utilities|String|ToString(Integer) _missionid)) true true "(R=0.000000,G=0.660000,B=1.000000,A=1.000000)" 1e+03)
    (Development|PrintString (Utilities|String|Append "CurrentTime: " (Utilities|String|ToString(Float) (Utilities|Array|Get(acopy) (Variables|Default|GetCurrentTime)))) true true "(R=0.000000,G=0.660000,B=1.000000,A=1.000000)" 1e+03)
    (Development|PrintString (Utilities|String|Append "Active: " (Utilities|String|ToString(Boolean) (Utilities|Array|Get(acopy) (Variables|Default|GetTimerActive)))) true true "(R=0.000000,G=0.660000,B=1.000000,A=1.000000)" 1e+03)
    (Math|Integer|IncrementInt (Variables|Default|GetTimersActiveAmmount))))

(fn SetTimer
  (params (Mission :type STRUCT%20Mission%20Settings%20Structure) (Time :type Float%20%28single-precision%29))
  (bind (_missionid _targetfood _targetclient _ordertime _ordercost _oderbenefit _odertype) (Utilities|Struct|BreakSTRUCT_MissionSettings Mission))
  (Default|SetTimer (Variables|Default|GetWidget_Timer) Time _missionid _odertype))

(fn GetMoney
  (return (Variables|Default|GetCurrentMoney)))