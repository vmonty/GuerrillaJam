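; BP_MenuController runs the game's start, pause and game-over menus, each built from WB_MenuController at BeginPlay.
; PopMenu shows or hides a menu and pauses or unpauses the game with it.
; GM_Guerrilla's MissionManager triggers game over with a summary, and the timer widget stays hidden until Begin.
; Accept and vertical input go to all three menus, with DoOnce latches turning axis input into single steps.
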(event Custom|QuitGame
  (Game|QuitGame 0 "Quit"))

(event Custom|ResumeGame
  (CallFunction|PopMenu (Variables|Default|GetPauseMenu) false))

(event Custom|RestartGame
  (Game|OpenLevel(byName) "LEVEL_Main"))

(event Custom|BeginGame
  (CallFunction|PopMenu (Variables|Default|GetStartMenu) false)
  (UserInterface|Viewport|AddtoViewport (Variables|/Game/Blueprints/PlayerSetup/GM_Guerrilla.GM_Guerrilla_C|GetWidget_Timer (.AsGM%20Guerrilla (Utilities|Casting|CastToGM_Guerrilla (Game|GetGameMode)))) 0))

(event Custom|Game%20Over
  (params (MissionSummary :type Text))
  (bind _gameovermenu (Variables|Default|GetGameOverMenu))
  (Rendering|Components|TextRender|SetText (Variables|/Game/UI/WB_MenuController.WB_MenuController_C|GetSubtitle_Text _gameovermenu) MissionSummary)
  (CallFunction|PopMenu _gameovermenu true))

(event EventBeginPlay
  (Utilities|FlowControl|Sequence
    (:then_0
      (bind _returnvalue (UserInterface|CreateWidget "/Game/UI/WB_MenuController.WB_MenuController_C" 0 "/Game/UI/WB_GameLogo.WB_GameLogo_C" false "Pause" " " "Resume" "Quit"))
      (bind _output_get (Variables|Default|SetPauseMenu _returnvalue))
      (EventDispatchers|AssignButton2Press _output_get (delegate Custom|QuitGame))
      (EventDispatchers|AssignButton1Press (Variables|Default|GetPauseMenu) (delegate Custom|ResumeGame)))
    (:then_1
      (bind _returnvalue_2 (UserInterface|CreateWidget "/Game/UI/WB_MenuController.WB_MenuController_C" 0 "/Game/UI/WB_GameLogo.WB_GameLogo_C" false "Game Over" "Congratulations! You've earned enough to buy a half-eatern Snickers." "Restart" "Quit"))
      (bind _output_get_2 (Variables|Default|SetGameOverMenu _returnvalue_2))
      (EventDispatchers|AssignButton2Press _output_get_2 (delegate Custom|QuitGame))
      (EventDispatchers|AssignButton1Press (Variables|Default|GetGameOverMenu) (delegate Custom|RestartGame))
      (bind _asgm_guerrilla (Utilities|Casting|CastToGM_Guerrilla (Game|GetGameMode)))
      (EventDispatchers|BindEventtoAllMissionFinished (Variables|/Game/Blueprints/PlayerSetup/GM_Guerrilla.GM_Guerrilla_C|GetMissionManager _asgm_guerrilla) (delegate Custom|Game%20Over)))
    (:then_2
      (bind _returnvalue_3 (UserInterface|CreateWidget "/Game/UI/WB_MenuController.WB_MenuController_C" 0 "/Game/UI/WB_GameLogo.WB_GameLogo_C" true "Devileroo" "Holy shit I hate this job. ;_;" "Begin" "Quit"))
      (bind _output_get_3 (Variables|Default|SetStartMenu _returnvalue_3))
      (EventDispatchers|AssignButton2Press _output_get_3 (delegate Custom|QuitGame))
      (EventDispatchers|AssignButton1Press (Variables|Default|GetStartMenu) (delegate Custom|BeginGame))
      (Utilities|FlowControl|Delay 0.2)
      (CallFunction|PopMenu (Variables|Default|GetStartMenu) true)
      (Widget|RemovefromParent (Variables|/Game/Blueprints/PlayerSetup/GM_Guerrilla.GM_Guerrilla_C|GetWidget_Timer (.AsGM%20Guerrilla (Utilities|Casting|CastToGM_Guerrilla (Game|GetGameMode))))))))

(event Input|ActionEvents|InputActionPause
  (params (Key :type Key%20Structure))
  (bind _pausemenu (Variables|Default|GetPauseMenu))
  (:Pressed
    (if (or (UserInterface|Viewport|IsinViewport (Variables|Default|GetGameOverMenu)) (UserInterface|Viewport|IsinViewport (Variables|Default|GetStartMenu)))
      (CallFunction|PopMenu _pausemenu false)
      (elif (not (UserInterface|Viewport|IsinViewport (Variables|Default|GetPauseMenu)))
        (CallFunction|PopMenu _pausemenu true)))))

(event Input|ActionEvents|InputActionAccept
  (params (Key :type Key%20Structure))
  (:Pressed
    (Default|ButtonAccept (Variables|Default|GetPauseMenu))))

(event Input|AxisEvents|InputAxisMenuUp
  (params (AxisValue :type Float%20%28single-precision%29))
  (bind _pausemenu (Variables|Default|GetPauseMenu))
  (Math|Float|CompareFloat AxisValue 0.0
    (:>
      (Utilities|FlowControl|DoOnce false :!label _label
        (:Completed
          (Default|VerticalInput _pausemenu "Forward"))))
    (:==
      (Utilities|FlowControl|Sequence
        (:then_0
          (goto _label Reset))
        (:then_1
          (goto _label_2 Reset))))
    (:<
      (Utilities|FlowControl|DoOnce false :!label _label_2
        (:Completed
          (Default|VerticalInput _pausemenu "Backward"))))))

(fn ConstructionScript)

(fn PopMenu
  (params (Menu%20Widget :type WB%20Menu%20Controller%20Object%20Reference) (Visible :type Boolean))
  (Game|SetGamePaused Visible)
  (if Visible
    (UserInterface|Viewport|AddtoViewport Menu%20Widget 0)
    (Default|FocusButton Menu%20Widget)
    (else
      (Widget|RemovefromParent Menu%20Widget))))