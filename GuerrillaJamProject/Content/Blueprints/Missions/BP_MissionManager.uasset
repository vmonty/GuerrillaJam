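; Mission manager for a food delivery game, tracking each order from pickup to delivery or failure and its effect on player money.
; BeginPlay assigns IDs to each mission's food and client actors, binds their interaction events and creates timer widgets through GM_Guerrilla.
; ChangeMissionState is the central switch, enabling triggers, updating money, timers and mission text, and broadcasting state changes.
; Once all missions finish, it broadcasts a money-based Devileroo summary.
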(event Custom|InteractionComplete
  (params (InteractionPlace :type BP%20Interaction%20Place%20Object%20Reference) (MissionID :type Integer))
  (switch Utilities|FlowControl|Switch|SwitchonENUM_InteractionPlace (Variables|/Game/Blueprints/Interaction/BP_InteractionPlace.BP_InteractionPlace_C|GetInteractionPlaceType InteractionPlace)
    (:NewEnumerator0
      (CallFunction|ChangeMissionState (Utilities|Array|Get(acopy) (Variables|Default|GetMissionList) MissionID) "NewEnumerator1"))
    (:NewEnumerator1
      (CallFunction|ChangeMissionState (Utilities|Array|Get(acopy) (Variables|Default|GetMissionList) MissionID) "NewEnumerator2"))))

(event Custom|InteractionImposible
  (params (InteractionPlace :type BP%20Interaction%20Place%20Object%20Reference) (MissionID :type Integer))
  (if (Utilities|Enum|NotEqual(Enum) (Variables|/Game/Blueprints/Interaction/BP_InteractionPlace.BP_InteractionPlace_C|GetInteractionPlaceState InteractionPlace) "NewEnumerator3")
    (Variables|/Game/Blueprints/Interaction/BP_InteractionPlace.BP_InteractionPlace_C|SetInteractionPlaceState InteractionPlace (Variables|/Game/Blueprints/Interaction/BP_InteractionPlace.BP_InteractionPlace_C|GetInteractionPlaceState InteractionPlace))
    (Development|PrintString "Hello")))

(event Custom|CustomEvent_0
  (params (MissionSummary :type Text))
  (Development|PrintString (Utilities|String|ToString(Text) MissionSummary) true true "(R=0.000000,G=0.660000,B=1.000000,A=1.000000)" 2e+07))

(event EventBeginPlay
  (EventDispatchers|BindEventtoAllMissionFinished (delegate Custom|CustomEvent_0))
  (bind _asgm_guerrilla (Utilities|Casting|CastToGM_Guerrilla (Game|GetGameMode)))
  (Variables|Default|SetGameMode _asgm_guerrilla)
  (for (_array_element _array_index) (Variables|Default|GetMissionList)
    (Default|SetMissionID (.TargetFood (Utilities|Struct|BreakSTRUCT_MissionSettings _array_element)) _array_index)
    (Default|SetMissionID (.TargetClient (Utilities|Struct|BreakSTRUCT_MissionSettings _array_element)) _array_index)
    (EventDispatchers|BindEventtoInteractionComplete (.TargetFood (Utilities|Struct|BreakSTRUCT_MissionSettings _array_element)) (delegate Custom|InteractionComplete))
    (EventDispatchers|BindEventtoInteractionComplete (.TargetClient (Utilities|Struct|BreakSTRUCT_MissionSettings _array_element)) (delegate Custom|InteractionComplete))
    (EventDispatchers|BindEventtoInteractionImposible (.TargetFood (Utilities|Struct|BreakSTRUCT_MissionSettings _array_element)) (delegate Custom|InteractionImposible))
    (EventDispatchers|BindEventtoInteractionImposible (.TargetClient (Utilities|Struct|BreakSTRUCT_MissionSettings _array_element)) (delegate Custom|InteractionImposible))
    (bind _returnvalue (UserInterface|CreateWidget "/Game/UI/WB_TimerBox.WB_TimerBox_C"))
    (bind _structout (Utilities|Struct|SetmembersinSTRUCT_MissionSettings _array_element _array_index _returnvalue))
    (Default|InitializeTimerWidget (Variables|Default|GetGameMode) _structout)))

(event Collision|EventActorBeginOverlap
  (params (OtherActor :type Actor%20Object%20Reference)))

(event EventTick
  (params (DeltaSeconds :type Float%20%28single-precision%29)))

(fn ConstructionScript)

(fn LaunchMissionbyIndex
  (params (Index :type Integer))
  (bind _missionlist (Variables|Default|GetMissionList))
  (bind _output (Utilities|Array|Get(acopy) _missionlist Index))
  (bind (_missionid _targetfood _targetclient _ordertime _ordercost _oderbenefit _odertype _orderstate) (Utilities|Struct|BreakSTRUCT_MissionSettings _output))
  (CallFunction|ChangeMissionState _output "NewEnumerator0")
  (Development|PrintString (Utilities|String|Append "DBG Mission launched id: " (Utilities|String|ToString(Integer) _missionid) "state" (Utilities|String|EnumtoString _orderstate)) true true "(R=1.000000,G=0.000000,B=0.000000,A=1.000000)" 1.2e+02))

(fn ChangeMissionState
  (params (Mission :type STRUCT%20Mission%20Settings%20Structure%20%28by%20ref%29) (State :type ENUM_MissionState%20Enum :default "NewEnumerator4"))
  (bind _output_get (LocalVariables|SetCurrentMission Mission))
  (bind _structout (Utilities|Struct|SetmembersinSTRUCT_MissionSettings _output_get State))
  (Development|PrintString (Utilities|String|Append "DBG Mission ID" (Utilities|String|ToString(Integer) (.MissionID (Utilities|Struct|BreakSTRUCT_MissionSettings _structout))) "changed to state" (Utilities|String|EnumtoString State)) true true "(R=1.000000,G=0.000000,B=0.000000,A=1.000000)" 1.2e+02)
  (Default|CallOrderStateChanged State (.MissionID (Utilities|Struct|BreakSTRUCT_MissionSettings _structout)))
  (Utilities|FlowControl|Sequence
    (:then_0
      (switch Utilities|FlowControl|Switch|SwitchonENUM_MissionState (.OrderState (Utilities|Struct|BreakSTRUCT_MissionSettings _structout))
        (:NewEnumerator0
          ;[1 1 1] Pick Item
          (CallFunction|LaunchWidget (.MissionText (Utilities|Struct|BreakSTRUCT_MissionSettings _structout)))
          (Default|EnableTrigger (.TargetFood (Utilities|Struct|BreakSTRUCT_MissionSettings (LocalVariables|GetCurrentMission))))
          (Default|PlayTimer (Variables|Default|GetGameMode) (LocalVariables|GetCurrentMission))
          ;[1 0 0] CHECK
          (Default|UpdateState (.TargetFood (Utilities|Struct|BreakSTRUCT_MissionSettings (LocalVariables|GetCurrentMission))) "NewEnumerator0"))
        (:NewEnumerator1
          ;[1 1 1] Picked Item
          (Default|EnableTrigger (.TargetClient (Utilities|Struct|BreakSTRUCT_MissionSettings (LocalVariables|GetCurrentMission))))
          (bind _asgm_guerrilla (Utilities|Casting|CastToGM_Guerrilla (Game|GetGameMode)))
          (Default|UpdateMoney _asgm_guerrilla (* -1 (.OrderCost (Utilities|Struct|BreakSTRUCT_MissionSettings (LocalVariables|GetCurrentMission)))))
          (Default|UpdateState (.TargetClient (Utilities|Struct|BreakSTRUCT_MissionSettings (LocalVariables|GetCurrentMission))) "NewEnumerator2"))
        (:NewEnumerator2
          ;[1 1 1] Delivered actions
          (bind _asgm_guerrilla_2 (Utilities|Casting|CastToGM_Guerrilla (Game|GetGameMode)))
          (Default|UpdateMoney _asgm_guerrilla_2 (* (.OrderCost (Utilities|Struct|BreakSTRUCT_MissionSettings (LocalVariables|GetCurrentMission))) (.OderBenefit (Utilities|Struct|BreakSTRUCT_MissionSettings (LocalVariables|GetCurrentMission)))))
          (Math|Integer|IncrementInt (Variables|Default|GetMissionFinishedCounter)
            (:%20%20
              (Default|HideTimer (Variables|Default|GetGameMode)))))
        (:NewEnumerator5
          ;[1 1 1] Destroy missions actors
          (Utilities|IsValid (.TargetFood (Utilities|Struct|BreakSTRUCT_MissionSettings (LocalVariables|GetCurrentMission)))
            (:Is%20Valid
              (Actor|DestroyActor (.TargetFood (Utilities|Struct|BreakSTRUCT_MissionSettings (LocalVariables|GetCurrentMission)))))
            (:Is%20Not%20Valid
              _))
          (Utilities|IsValid (.TargetClient (Utilities|Struct|BreakSTRUCT_MissionSettings (LocalVariables|GetCurrentMission)))
            (:Is%20Valid
              (Actor|DestroyActor (.TargetClient (Utilities|Struct|BreakSTRUCT_MissionSettings (LocalVariables|GetCurrentMission))))
              (Math|Integer|IncrementInt (Variables|Default|GetMissionFinishedCounter)))))))
    (:then_1
      (if (== (Utilities|Array|Length (Variables|Default|GetMissionList)) (Variables|Default|GetMissionFinishedCounter))
        (bind _missionsummary (CallFunction|GetMissionSummary))
        (Default|CallAllMissionFinished _missionsummary)))))

(fn LaunchWidget
  (params (Message :type Text))
  (Development|PrintString (Utilities|String|ToString(Text) Message))
  (Utilities|IsValid (Variables|Default|GetMissionWidget)
    (:Is%20Valid
      _)
    (:Is%20Not%20Valid
      (bind _returnvalue (UserInterface|CreateWidget "/Game/UI/WB_MissionInfo.WB_MissionInfo_C"))
      (bind _output_get (Variables|Default|SetMissionWidget _returnvalue))
      (UserInterface|Viewport|AddtoViewport _output_get 0)))
  (Development|PrintString (Utilities|String|ToString(Text) Message))
  (Variables|/Game/UI/WB_MissionInfo.WB_MissionInfo_C|SetLastMissionText (Variables|Default|GetMissionWidget) Message))

(fn MissionFailed
  (params (Mission :type STRUCT%20Mission%20Settings%20Structure%20%28by%20ref%29))
  (CallFunction|ChangeMissionState Mission "NewEnumerator5"))

(fn GetMissionSummary
  (bind _currentmoney (Default|GetMoney (Variables|Default|GetGameMode)))
  (LocalVariables|SetMoneyText (Utilities|Text|ToText(Float) _currentmoney "HalfToEven" false true 1 324 0 2))
  (Math|Float|CompareFloat _currentmoney 0.0
    (:>
      (bind _newparam (CallFunction|GetAffordableFood _currentmoney :!label _label))
      (LocalVariables|SetSummaryText (Utilities|Text|ToText(String) (Utilities|String|Append "Devileroo thanks your effort. Today you could afford" (Utilities|String|ToString(Text) _newparam) " with those " (Utilities|String|ToString(Text) (LocalVariables|GetMoneyText)) "$"))))
    (:==
      (goto _label))
    (:<
      (LocalVariables|SetSummaryText (Utilities|Text|ToText(String) (Utilities|String|Append "You owe Devileroo " (Utilities|String|ToString(Text) (LocalVariables|GetMoneyText)) "$")))))
  (return (LocalVariables|GetSummaryText)))

(fn GetAffordableFood
  (params (Money :type Float%20%28single-precision%29))
  (Utilities|FlowControl|Sequence
    (:then_0
      (Math|Float|CompareFloat Money 1.0
        (:>
          (Math|Float|CompareFloat Money 5.0
            (:>
              (Math|Float|CompareFloat Money 1e+01
                (:>
                  (Math|Float|CompareFloat Money 2e+01
                    (:>
                      (LocalVariables|SetText "  Lobster"))
                    (:==
                      (LocalVariables|SetText "  a whole Burguer and an Ice Cream" :!label _label))
                    (:<
                      (goto _label))))
                (:==
                  (LocalVariables|SetText "  a whole Burguer" :!label _label_2))
                (:<
                  (goto _label_2))))
            (:==
              (LocalVariables|SetText "  half Burguer" :!label _label_3))
            (:<
              (goto _label_3))))
        (:==
          (LocalVariables|SetText " a Coffe" :!label _label_4))
        (:<
          (goto _label_4))))
    (:then_1
      (return (LocalVariables|GetText)))))