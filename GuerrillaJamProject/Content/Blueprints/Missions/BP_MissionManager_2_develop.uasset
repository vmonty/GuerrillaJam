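; Mission manager actor that runs pickup-and-delivery food orders between a food spot and a client.
; On BeginPlay it tags each mission's targets with its index, binds their interaction events and hands a timer widget to GM_Guerrilla.
; A state switch enables triggers, starts the timer, charges the order cost on pickup, pays out on delivery and destroys targets on failure.
; Mission messages and the impossible-interaction handler are only debug prints.
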(event Custom|InteractionComplete
  (params (InteractionPlace :type BP%20Interaction%20Place%20Object%20Reference) (MissionID :type Integer))
  (switch Utilities|FlowControl|Switch|SwitchonENUM_InteractionPlace (Variables|/Game/Blueprints/Interaction/BP_InteractionPlace.BP_InteractionPlace_C|GetInteractionPlaceType InteractionPlace)
    (:NewEnumerator0
      (CallFunction|ChangeMissionState (Utilities|Array|Get(acopy) (Variables|Default|GetMissionList) MissionID) "NewEnumerator1"))
    (:NewEnumerator1
      (CallFunction|ChangeMissionState (Utilities|Array|Get(acopy) (Variables|Default|GetMissionList) MissionID) "NewEnumerator2"))))

(event Custom|InteractionImposible
  (params (InteractionPlace :type BP%20Interaction%20Place%20Object%20Reference) (MissionID :type Integer))
  (if (Utilities|Enum|NotEqual(Enum) (Variables|/Game/Blueprints/Interaction/BP_InteractionPlace.BP_InteractionPlace_C|GetInteractionPlaceState InteractionPlace) "NewEnumerator3")
    (Variables|/Game/Blueprints/Interaction/BP_InteractionPlace.BP_InteractionPlace_C|SetInteractionPlaceState InteractionPlace (Variables|/Game/Blueprints/Interaction/BP_InteractionPlace.BP_InteractionPlace_C|GetInteractionPlaceState InteractionPlace))
    (Development|PrintString "Hello")))

(event EventBeginPlay
  (bind _asgm_guerrilla (Utilities|Casting|CastToGM_Guerrilla (Game|GetGameMode)))
  (Variables|Default|SetGameMode _asgm_guerrilla)
  (for (_array_element _array_index) (Variables|Default|GetMissionList)
    (Default|SetMissionID (.TargetFood (Utilities|Struct|BreakSTRUCT_MissionSettings _array_element)) _array_index)
    (Default|SetMissionID (.TargetClient (Utilities|Struct|BreakSTRUCT_MissionSettings _array_element)) _array_index)
    (EventDispatchers|BindEventtoInteractionComplete (.TargetFood (Utilities|Struct|BreakSTRUCT_MissionSettings _array_element)) (delegate Custom|InteractionComplete))
    (EventDispatchers|BindEventtoInteractionComplete (.TargetClient (Utilities|Struct|BreakSTRUCT_MissionSettings _array_element)) (delegate Custom|InteractionComplete))
    (EventDispatchers|BindEventtoInteractionImposible (.TargetFood (Utilities|Struct|BreakSTRUCT_MissionSettings _array_element)) (delegate Custom|InteractionImposible))
    (EventDispatchers|BindEventtoInteractionImposible (.TargetClient (Utilities|Struct|BreakSTRUCT_MissionSettings _array_element)) (delegate Custom|InteractionImposible))
    (bind _returnvalue (UserInterface|CreateWidget "/Game/UI/WB_TimerBox.WB_TimerBox_C"))
    (bind _structout (Utilities|Struct|SetmembersinSTRUCT_MissionSettings _array_element _array_index _returnvalue))
    (Default|InitializeTimerWidget (Variables|Default|GetGameMode) _structout)))

(event Collision|EventActorBeginOverlap
  (params (OtherActor :type Actor%20Object%20Reference)))

(event EventTick
  (params (DeltaSeconds :type Float%20%28single-precision%29)))

(fn ConstructionScript)

(fn LaunchMissionbyIndex
  (params (Index :type Integer))
  (CallFunction|ChangeMissionState (Utilities|Array|Get(acopy) (Variables|Default|GetMissionList) Index) "NewEnumerator0"))

(fn ChangeMissionState
  (params (Mission :type STRUCT%20Mission%20Settings%20Structure%20%28by%20ref%29) (State :type ENUM_MissionState%20Enum :default "NewEnumerator4"))
  (bind _output_get (LocalVariables|SetCurrentMission Mission))
  (Utilities|Struct|SetmembersinSTRUCT_MissionSettings _output_get State)
  (switch Utilities|FlowControl|Switch|SwitchonENUM_MissionState State
    (:NewEnumerator0
      ;[1 1 1] Pick Item
      (CallFunction|LaunchWidget "Mission start")
      (Default|EnableTrigger (.TargetFood (Utilities|Struct|BreakSTRUCT_MissionSettings (LocalVariables|GetCurrentMission))))
      (Default|PlayTimer (Variables|Default|GetGameMode) (LocalVariables|GetCurrentMission))
      ;[1 0 0] CHECK
      (Default|UpdateState (.TargetFood (Utilities|Struct|BreakSTRUCT_MissionSettings (LocalVariables|GetCurrentMission))) "NewEnumerator0"))
    (:NewEnumerator1
      ;[1 1 1] Picked Item
      (CallFunction|LaunchWidget "Item picked")
      (Default|EnableTrigger (.TargetClient (Utilities|Struct|BreakSTRUCT_MissionSettings (LocalVariables|GetCurrentMission))))
      (bind _asgm_guerrilla (Utilities|Casting|CastToGM_Guerrilla (Game|GetGameMode)))
      (Default|UpdateMoney _asgm_guerrilla (* -1 (.OrderCost (Utilities|Struct|BreakSTRUCT_MissionSettings (LocalVariables|GetCurrentMission)))))
      (Default|UpdateState (.TargetClient (Utilities|Struct|BreakSTRUCT_MissionSettings (LocalVariables|GetCurrentMission))) "NewEnumerator0" "NewEnumerator2"))
    (:NewEnumerator2
      ;[1 1 1] Delivered actions
      (bind _asgm_guerrilla_2 (Utilities|Casting|CastToGM_Guerrilla (Game|GetGameMode)))
      (Default|UpdateMoney _asgm_guerrilla_2 (* (.OrderCost (Utilities|Struct|BreakSTRUCT_MissionSettings (LocalVariables|GetCurrentMission))) (.OderBenefit (Utilities|Struct|BreakSTRUCT_MissionSettings (LocalVariables|GetCurrentMission))))))
    (:NewEnumerator5
      ;[1 1 1] Destroy missions actors
      (Utilities|IsValid (.TargetFood (Utilities|Struct|BreakSTRUCT_MissionSettings (LocalVariables|GetCurrentMission)))
        (:Is%20Valid
          (Actor|DestroyActor (.TargetFood (Utilities|Struct|BreakSTRUCT_MissionSettings (LocalVariables|GetCurrentMission)))))
        (:Is%20Not%20Valid
          _))
      (Utilities|IsValid (.TargetClient (Utilities|Struct|BreakSTRUCT_MissionSettings (LocalVariables|GetCurrentMission)))
        (:Is%20Valid
          (Actor|DestroyActor (.TargetClient (Utilities|Struct|BreakSTRUCT_MissionSettings (LocalVariables|GetCurrentMission)))))))))

(fn LaunchWidget
  (params (Message :type Text))
  (Development|PrintString (Utilities|String|ToString(Text) Message)))

(fn MissionFailed
  (params (Mission :type STRUCT%20Mission%20Settings%20Structure%20%28by%20ref%29))
  (CallFunction|ChangeMissionState Mission "NewEnumerator5"))